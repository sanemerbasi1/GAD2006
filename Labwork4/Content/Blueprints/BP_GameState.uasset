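; Game state Blueprint that resolves a team match between Blue and Red and shows the result on screen.
; On victory it tells each player's avatar it won or lost: Blue wins if the timer has ended, otherwise Red wins.
; It then creates a results widget showing a loss message or the winning player's nickname, based on the local player's result.
; On restart it removes that widget.
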(event `self.OnVictory`
  (for _array_element (`self.PlayerArray`)
    (bind _asnet_player_state (cast `NetPlayerState` _array_element))
    (bind (_data_nickname _data_customizationdata _data_teamid) (break `SPlayerInfo` (`NetPlayerState.Data` _asnet_player_state)))
    (switch `EPlayerTeam` _data_teamid
      (:`TEAM_Blue`
        (if (`self.TimerEnd`)
          (bind _asbp_net_avatar (cast `/Game/Blueprints/BP_NetAvatar` (`PlayerState.PawnPrivate` _asnet_player_state) :!pure true))
          (`/Game/Blueprints/BP_NetAvatar.OnPlayerWon` _asbp_net_avatar :!label _label)
          (else
            (`/Game/Blueprints/BP_NetAvatar.OnPlayerLost` _asbp_net_avatar :!label _label_2))))
      (:`TEAM_Red`
        (if (`self.TimerEnd`)
          (goto _label_2)
          (else
            (goto _label))))))
  (`self.Show Result Message`))

(event `self.OnRestart`
  (`Widget.RemoveFromParent` (`self.Message Widget`)))

(fn `Show Result Message`
  (bind _returnvalue (`self.GetPlayerStateByIndex` (`self.WinningPlayer`)))
  (bind _returnvalue_2 (`|CreateWidget` "/Game/Blueprints/UMG/W_GameResults.W_GameResults_C" null (select `bool` (`|EnumEquality` (`NetPlayerState.Result` (cast `NetPlayerState` (`Controller.PlayerState` (`GameplayStatics.GetPlayerController` 0)) :!pure true)) "RESULT_Lost") :`false` (`|FormatText` "{Name} WINS!" (`.Nickname` (break `SPlayerInfo` (`NetPlayerState.Data` _returnvalue)))) :`true` "YOU LOSE!")))
  (set `self.Message Widget` _returnvalue_2)
  (`UserWidget.AddToViewport` _returnvalue_2 0))

(fn `UserConstructionScript`)